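; VR player pawn for the LoftOffice project, with floor-origin tracking, teleport, snap turn and smooth locomotion.
; Holding Teleport traces a projectile arc from the right controller with debug drawing and a destination arrow; release teleports if the last hit surface was flat enough.
; Stick input past a deadzone moves along camera forward or snap-turns the Scene component once per push via DoOnce.
; Grip inputs only set left and right fist flags.
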(event `self.ReceiveTick`
  (params (DeltaSeconds :type "Float (single-precision)"))
  ;[1 1 1] Teleport
  (if (`self.Teleport`)
    (`self.TeleportTRace`)))

(event `self.ReceiveBeginPlay`
  ;[1 1 1] LocationCamera
  (`HeadMountedDisplayFunctionLibrary.SetTrackingOrigin` "Floor"))

(event `InputAction|Teleport`
  (params (Key :type "Key Structure"))
  ;[1 1 1] Teleport
  (:`Pressed`
    (set `self.Teleport` true))
  (:`Released`
    (set `self.Teleport` false)
    (`SceneComponent.SetHiddenInGame` (`self.TeleportArrowRotation`) true false)
    (if (`self.CanTeleport`)
      (`self.K2_TeleportTo` (`self.TeleportLocation`) (`self.K2_GetActorRotation`)))))

(event `InputAction|GrapRightFist`
  (params (Key :type "Key Structure"))
  ;[1 1 1] AnimtionPickUp
  (:`Pressed`
    (set `self.RightMakeFist` true))
  (:`Released`
    (set `self.RightMakeFist` false)))

(event `InputAction|GrapLightFist`
  (params (Key :type "Key Structure"))
  ;[1 1 1] AnimtionPickUp
  (:`Pressed`
    (set `self.LightMakeFist` true))
  (:`Released`
    (set `self.LightMakeFist` false)))

(event `InputAxis|Turn`
  (params (AxisValue :type "Float (single-precision)"))
  ;[1 1 1] Turn around
  (if (`self.Is Axis greater than Deadzone` AxisValue)
    (`/Engine/EditorBlueprintResources/StandardMacros.DoOnce` false :!label _label
      (:`Completed`
        (`self.Turn` (< AxisValue 0.0))))
    (else
      (goto _label :!via `Reset`))))

(event `InputAxis|Move`
  (params (AxisValue :type "Float (single-precision)"))
  ;[1 1 1] Movement
  (if (`self.Is Axis greater than Deadzone` AxisValue)
    (`self.AddMovementInput` (`SceneComponent.GetForwardVector` (`self.Camera`)) (* AxisValue (`self.MovementScaler`)))))

(fn `Is Axis greater than Deadzone`
  (params (Input :type "Float (double-precision)"))
  (returns (Return :type Boolean))
  (return (>= (`KismetMathLibrary.Abs` Input) (`self.AxisDeadZone`))))

(fn `TeleportTRace`
  (bind _teleportarrowrotation (`self.TeleportArrowRotation`))
  (bind _rightmc (`self.RightMC`))
  (bind (_outhit _outpathpositions _outlasttracedestination _returnvalue) (`GameplayStatics.Blueprint_PredictProjectilePath_ByObjectType` :`StartPos` (`SceneComponent.K2_GetComponentLocation` _rightmc) :`LaunchVelocity` (* (`KismetMathLibrary.GetForwardVector` (`SceneComponent.K2_GetComponentRotation` _rightmc)) (`self.TeleportTraceLength`)) :`ProjectileRadius` 10.0 :`ObjectTypes` (`|MakeArray` "ObjectTypeQuery1" "ObjectTypeQuery2" :!type "EObjectTypeQuery Enum") :`DrawDebugType` "ForDuration" :`SimFrequency` 20.0))
  (if _returnvalue
    (bind (_bblockinghit _binitialoverlap _time _distance _location _impactpoint _normal _impactnormal) (`GameplayStatics.BreakHitResult` _outhit))
    (set `self.CanTeleport` (>= (.z _impactnormal) 0.5))
    (bind _output_get (set `self.TeleportLocation` _impactpoint))
    (`KismetSystemLibrary.DrawDebugCylinder` _output_get (+ _output_get (0.0 0.0 50.0)) 20.0 20)
    (`SceneComponent.SetHiddenInGame` _teleportarrowrotation false false)
    (`SceneComponent.K2_SetWorldLocation` _teleportarrowrotation (`self.TeleportLocation`) false false)
    (else
      (`SceneComponent.SetHiddenInGame` (`self.TeleportArrowRotation`) true false))))

(fn `Turn`
  (params (`Is Left ?` :type Boolean))
  (`SceneComponent.K2_SetWorldRotation` (`self.Scene`) (`KismetMathLibrary.ComposeRotators` (`SceneComponent.K2_GetComponentRotation` (`self.Scene`)) (`KismetMathLibrary.MakeRotator` 0.0 0.0 (`KismetMathLibrary.SelectFloat` -15.0 15.0 `Is Left ?`))) false false)
  (`KismetSystemLibrary.PrintString` (`KismetStringLibrary.Concat_StrStr` "Rotate: " (`KismetStringLibrary.Conv_RotatorToString` (struct)))))

(fn `UserConstructionScript`)