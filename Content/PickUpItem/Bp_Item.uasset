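; Pickup item Blueprint that can be attached to a carrier and shows a world-space widget prompt.
; InteracPicUp snaps its StaticMesh to the "Socket" socket of the passed component.
; For actors not tagged "Door", TraceAChangeMaterial toggles the widget's visibility and turns it once per call to face the player's BP_Character camera.
; Despite that event's name, it changes no material.
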(event `/Game/PickUpItem/InterfaceInterac.InteracPicUp`
  (params (`Attach to` :type "SceneComponent Object Reference"))
  (`SceneComponent.K2_AttachToComponent` (`self.StaticMesh`) `Attach to` "Socket" "SnapToTarget" "SnapToTarget" "SnapToTarget" true))

(event `/Game/PickUpItem/InterfaceInterac.TraceAChangeMaterial`
  (bind _widget (`self.Widget`))
  (if (not (`self.ActorHasTag` "Door"))
    (`SceneComponent.ToggleVisibility` _widget false)
    (bind _asbp_character (cast `/Game/Test_Teleport/BP_Character` (`GameplayStatics.GetPlayerCharacter` 0)))
    (`SceneComponent.K2_SetWorldRotation` _widget (`KismetMathLibrary.MakeRotator` (* (.roll (`SceneComponent.K2_GetComponentRotation` (`/Game/Test_Teleport/BP_Character.Camera` _asbp_character))) -1.0) (* (.pitch (`SceneComponent.K2_GetComponentRotation` (`/Game/Test_Teleport/BP_Character.Camera` _asbp_character))) -1.0) (+ (.yaw (`SceneComponent.K2_GetComponentRotation` (`/Game/Test_Teleport/BP_Character.Camera` _asbp_character))) 180.0)) false false)))

(fn `UserConstructionScript`)