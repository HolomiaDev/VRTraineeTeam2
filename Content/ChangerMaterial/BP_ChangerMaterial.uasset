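; BP_ChangerMaterial is an interactable that shows or hides a material widget, apparently for changing materials.
; On BeginPlay it sets itself as the Owner of the WidGet_material hosted in its Widget component.
; InteractionMaterial toggles that component's visibility, then turns it once to face the BP_Character camera by negating pitch and roll and adding 180 degrees to yaw.
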(event `self.ReceiveBeginPlay`
  (bind _aswid_get_material (cast `/Game/ChangerMaterial/WidGet_material` (`WidgetComponent.GetUserWidgetObject` (`self.Widget`))))
  (set `/Game/ChangerMaterial/WidGet_material.Owner` self _aswid_get_material))

(event `/Game/ChangerMaterial/Interaction_Material.InteractionMaterial`
  (bind _widget (`self.Widget`))
  (`SceneComponent.ToggleVisibility` _widget false)
  (bind _asbp_character (cast `/Game/Test_Teleport/BP_Character` (`GameplayStatics.GetPlayerCharacter` 0)))
  (bind (_returnvalue_roll _returnvalue_pitch _returnvalue_yaw) (`KismetMathLibrary.BreakRotator` (`SceneComponent.K2_GetComponentRotation` (`/Game/Test_Teleport/BP_Character.Camera` _asbp_character))))
  (`SceneComponent.K2_SetWorldRotation` _widget (`KismetMathLibrary.MakeRotator` (* _returnvalue_roll -1.0) (* _returnvalue_pitch -1.0) (+ _returnvalue_yaw 180.0)) false false))

(fn `UserConstructionScript`)