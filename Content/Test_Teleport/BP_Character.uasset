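; VR test character that previews a teleport arc from the right motion controller while the Teleport input is held.
; Pressing and releasing the input toggles a flag that Tick checks to run TeleportTRace.
; The trace predicts a projectile path along the controller's forward vector against static and dynamic world objects, with per-frame debug drawing.
; It only prints hit point and normals; no teleport move is performed.
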(event `self.ReceiveBeginPlay`
  (`SceneComponent.SetWorldScale3D` (`self.RightHand`) (1.0 1.0 1.0)))

(event `self.ReceiveTick`
  (params (DeltaSeconds :type "Float (single-precision)"))
  (if (`self.Teleport`)
    (`self.TeleportTRace`)))

(event `InputAction|Teleport`
  (params (Key :type "Key Structure"))
  (:`Pressed`
    (set `self.Teleport` true))
  (:`Released`
    (set `self.Teleport` false)))

(fn `TeleportTRace`
  (bind _rightmc (`self.RightMC`))
  (bind _outhit (`GameplayStatics.Blueprint_PredictProjectilePath_ByObjectType` :`StartPos` (`SceneComponent.K2_GetComponentLocation` _rightmc) :`LaunchVelocity` (* (`KismetMathLibrary.GetForwardVector` (`SceneComponent.K2_GetComponentRotation` _rightmc)) (`self.TeleportTraceLength`)) :`ProjectileRadius` 10.0 :`ObjectTypes` (`|MakeArray` "ObjectTypeQuery1" "ObjectTypeQuery2" :!type "EObjectTypeQuery Enum") :`DrawDebugType` "ForOneFrame"))
  (bind (_bblockinghit _binitialoverlap _time _distance _location _impactpoint _normal _impactnormal) (`GameplayStatics.BreakHitResult` _outhit))
  (`KismetSystemLibrary.PrintString` (`KismetStringLibrary.Concat_StrStr` "ImpactNormal: " (`KismetStringLibrary.Conv_VectorToString` _impactpoint) "Loaction: " (`KismetStringLibrary.Conv_VectorToString` _normal) "Impactnormal: " (`KismetStringLibrary.Conv_VectorToString` _impactnormal))))

(fn `UserConstructionScript`)